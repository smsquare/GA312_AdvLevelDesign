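; BP_SceneAsset is a reusable set-dressing actor that shows one of several props, such as crates, lockers, a sconce or a TV.
; Its construction script switches on the TypeOfSceneAsset value and assigns the matching static mesh to the Mesh component.
; The event graph holds only disabled placeholder events, so the actor has no runtime logic.
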(event EventBeginPlay)

(event Collision|EventActorBeginOverlap
  (params (OtherActor :type Actor%20Object%20Reference)))

(event EventTick
  (params (DeltaSeconds :type Float%20%28single-precision%29)))

(fn ConstructionScript
  (switch Utilities|FlowControl|Switch|SwitchonESceneAssetType (Variables|Default|GetTypeOfSceneAsset)
    (:NewEnumerator0
      (Components|StaticMesh|SetStaticMesh (Variables|Default|GetMesh) "/Game/Geometry/Meshes/SceneAssets/MESH_Crate01.MESH_Crate01"))
    (:NewEnumerator1
      (Components|StaticMesh|SetStaticMesh (Variables|Default|GetMesh) "/Game/Geometry/Meshes/SceneAssets/MESH_Crate02.MESH_Crate02"))
    (:NewEnumerator4
      (Components|StaticMesh|SetStaticMesh (Variables|Default|GetMesh) "/Game/Geometry/Meshes/SceneAssets/MESH_Lockers.MESH_Lockers"))
    (:NewEnumerator3
      (Components|StaticMesh|SetStaticMesh (Variables|Default|GetMesh) "/Game/Geometry/Meshes/SceneAssets/MESH_Sconce.MESH_Sconce"))
    (:NewEnumerator2
      (Components|StaticMesh|SetStaticMesh (Variables|Default|GetMesh) "/Game/Geometry/Meshes/SceneAssets/MESH_TV.MESH_TV"))))